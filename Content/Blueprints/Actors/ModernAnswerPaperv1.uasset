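; Scoreboard paper actor for the elemental dice fight, meant to show hero and enemy values per round, totals and element icons.
; Only Reset does work, zeroing both totals (CorrectAnswers, WrongAnswers); UpdatePaper and the construction script are empty.
; The display logic is disconnected and never runs: it reads DiceFightGameMode elements and rounds, alternating turns via OpponentsRound.
; Other dead chains pick the enemy element by branching on EnemyElement.
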(event `Reset`
  (set `self.CorrectAnswers` 0)
  (set `self.WrongAnswers` 0))

(event `UpdatePaper`)

(fn `UserConstructionScript`)