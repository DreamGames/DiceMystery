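; Physics-simulated six-sided die actor that tracks which face it shows in a Value variable.
; BeginPlay enables physics on the Dice component, then Tick compares its relative rotation to right angles within ErrorTolerance.
; Near-zero pitch resolves 1, 2, 5 or 6 by roll, while other pitches resolve 3 or 4, with fallback tests reading Roll rather than Pitch.
; Unmatched orientations keep the previous Value, and no check waits for rest.
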(event `self.ReceiveBeginPlay`
  (`PrimitiveComponent.SetSimulatePhysics` (`self.Dice`) true))

(event `self.ReceiveTick`
  (params (DeltaSeconds :type "Float (single-precision)"))
  (bind _dice (`self.Dice`))
  (bind _dice_2 (`self.Dice`))
  (bind _dice_3 (`self.Dice`))
  (bind _dice_4 (`self.Dice`))
  (bind _dice_5 (`self.Dice`))
  (if (`KismetMathLibrary.NearlyEqual_FloatFloat` (.pitch (.rotation (`SceneComponent.GetRelativeTransform` (`self.Dice`)))) 0.0 (`self.ErrorTolerance`))
    (if (or (`KismetMathLibrary.NearlyEqual_FloatFloat` (.roll (.rotation (`SceneComponent.GetRelativeTransform` _dice_2))) 0.0 (`self.ErrorTolerance`)) (`KismetMathLibrary.NearlyEqual_FloatFloat` (.roll (.rotation (`SceneComponent.GetRelativeTransform` _dice_2))) 360.0 (`self.ErrorTolerance`)))
      (set `self.Value` 1)
      (elif (or (`KismetMathLibrary.NearlyEqual_FloatFloat` (.roll (.rotation (`SceneComponent.GetRelativeTransform` _dice_3))) 90.0 (`self.ErrorTolerance`)) (`KismetMathLibrary.NearlyEqual_FloatFloat` (.roll (.rotation (`SceneComponent.GetRelativeTransform` _dice_3))) -270.0 (`self.ErrorTolerance`)))
        (set `self.Value` 5)
        (elif (`KismetMathLibrary.NearlyEqual_FloatFloat` (`KismetMathLibrary.Abs` (.roll (.rotation (`SceneComponent.GetRelativeTransform` (`self.Dice`))))) 180.0 (`self.ErrorTolerance`))
          (set `self.Value` 6)
          (elif (or (`KismetMathLibrary.NearlyEqual_FloatFloat` (.roll (.rotation (`SceneComponent.GetRelativeTransform` _dice))) 270.0 (`self.ErrorTolerance`)) (`KismetMathLibrary.NearlyEqual_FloatFloat` (.roll (.rotation (`SceneComponent.GetRelativeTransform` _dice))) -90.0 (`self.ErrorTolerance`)))
            (set `self.Value` 2)))))
    (elif (or (`KismetMathLibrary.NearlyEqual_FloatFloat` (.pitch (.rotation (`SceneComponent.GetRelativeTransform` _dice_4))) 90.0 (`self.ErrorTolerance`)) (`KismetMathLibrary.NearlyEqual_FloatFloat` (.roll (.rotation (`SceneComponent.GetRelativeTransform` _dice_4))) -270.0 (`self.ErrorTolerance`)))
      (set `self.Value` 3)
      (elif (or (`KismetMathLibrary.NearlyEqual_FloatFloat` (.pitch (.rotation (`SceneComponent.GetRelativeTransform` _dice_5))) 270.0 (`self.ErrorTolerance`)) (`KismetMathLibrary.NearlyEqual_FloatFloat` (.roll (.rotation (`SceneComponent.GetRelativeTransform` _dice_5))) -90.0 (`self.ErrorTolerance`)))
        (set `self.Value` 4)))))

(fn `UserConstructionScript`)