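; Dice actor that reports which of three elements its resting orientation represents, with opposite orientations sharing a value.
; Every tick it compares the Dice component's relative pitch and roll to right angles within ErrorTolerance and sets Element, keeping the last value when nothing matches.
; The ReselLocation event snaps the Dice back to the DefaultSceneRoot transform.
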(event `ReselLocation`
  (`SceneComponent.K2_SetWorldTransform` (`self.Dice`) (`SceneComponent.K2_GetComponentToWorld` (`self.DefaultSceneRoot`)) false false))

(event `self.ReceiveTick`
  (params (DeltaSeconds :type "Float (single-precision)"))
  (bind _errortolerance (`self.ErrorTolerance`))
  (bind _errortolerance_2 (`self.ErrorTolerance`))
  (bind _errortolerance_3 (`self.ErrorTolerance`))
  (bind _errortolerance_4 (`self.ErrorTolerance`))
  (bind _errortolerance_5 (`self.ErrorTolerance`))
  (bind _returnvalue (`SceneComponent.GetRelativeTransform` (`self.Dice`)))
  (bind _returnvalue_2 (`SceneComponent.GetRelativeTransform` (`self.Dice`)))
  (bind _returnvalue_3 (`SceneComponent.GetRelativeTransform` (`self.Dice`)))
  (bind _returnvalue_4 (`SceneComponent.GetRelativeTransform` (`self.Dice`)))
  (bind _returnvalue_5 (`SceneComponent.GetRelativeTransform` (`self.Dice`)))
  (if (and (or (`KismetMathLibrary.NearlyEqual_FloatFloat` (.pitch (.rotation _returnvalue_4)) 0.0 _errortolerance_3) (`KismetMathLibrary.NearlyEqual_FloatFloat` (.pitch (.rotation _returnvalue_4)) 180.0 _errortolerance_3)) (or (`KismetMathLibrary.NearlyEqual_FloatFloat` (.roll (.rotation _returnvalue_5)) 0.0 _errortolerance_4) (`KismetMathLibrary.NearlyEqual_FloatFloat` (.roll (.rotation _returnvalue_5)) 180.0 _errortolerance_4)))
    (set `self.Element` 0)
    (elif (or (`KismetMathLibrary.NearlyEqual_FloatFloat` (.pitch (.rotation _returnvalue)) 90.0 _errortolerance_5) (`KismetMathLibrary.NearlyEqual_FloatFloat` (.pitch (.rotation _returnvalue)) -90.0 _errortolerance_5) (`KismetMathLibrary.NearlyEqual_FloatFloat` (.pitch (.rotation _returnvalue)) 270.0 _errortolerance_5))
      (set `self.Element` 1)
      (elif (and (or (`KismetMathLibrary.NearlyEqual_FloatFloat` (.pitch (.rotation _returnvalue_2)) 0.0 _errortolerance) (`KismetMathLibrary.NearlyEqual_FloatFloat` (.pitch (.rotation _returnvalue_2)) 180.0 _errortolerance)) (or (`KismetMathLibrary.NearlyEqual_FloatFloat` (.roll (.rotation _returnvalue_3)) 90.0 _errortolerance_2) (`KismetMathLibrary.NearlyEqual_FloatFloat` (.roll (.rotation _returnvalue_3)) -90.0 _errortolerance_2)))
        (set `self.Element` 2)))))

(fn `UserConstructionScript`)