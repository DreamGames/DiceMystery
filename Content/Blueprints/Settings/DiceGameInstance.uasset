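; Game instance for a dice game that persists games-played tallies and tutorial-played states for its Classic and two Modern modes.
; SaveGame and LoadGame copy these values to and from a DiceSaveGame object stored in the PlayedGamesInfo slot.
; A separate ToText event appends a round entry to a result string and writes it to a hardcoded desktop text file, overwriting it.
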(event `SaveGame`
  (`/Engine/EditorBlueprintResources/StandardMacros.IsValid` (`self.SaveGameInstance`)
    (:`Is Valid`
      _)
    (:`Is Not Valid`
      (bind _returnvalue (`GameplayStatics.CreateSaveGameObject` "/Game/Blueprints/Settings/DiceSaveGame.DiceSaveGame_C"))
      (bind _output_get (set `self.SaveGameInstance` _returnvalue))))
  (set `/Game/Blueprints/Settings/DiceSaveGame.TotalGamesPlayed` (`self.TotalGamesPlayed`) _output_get)
  (set `/Game/Blueprints/Settings/DiceSaveGame.ClassicGamesPlayed` (`self.ClassicGamesPlayed`) _output_get)
  (set `/Game/Blueprints/Settings/DiceSaveGame.ModernGamesPlayedv2` (`self.ModernGamesPlayedv2`) _output_get)
  (set `/Game/Blueprints/Settings/DiceSaveGame.ModernGamesPlayedv1` (`self.ModernGamesPlayedv1`) _output_get)
  (set `/Game/Blueprints/Settings/DiceSaveGame.ClassicTutorialPlayed?` (`self.ClassicTutorialPlayed?`) _output_get)
  (set `/Game/Blueprints/Settings/DiceSaveGame.ModernV1TutorialPlayed?` (`self.ModernV1TutorialPlayed?`) _output_get)
  (set `/Game/Blueprints/Settings/DiceSaveGame.ModernV2TutorialPlayed?` (`self.ModernV2TutorialPlayed?`) _output_get)
  (`GameplayStatics.SaveGameToSlot` _output_get "PlayedGamesInfo"))

(event `LoadGame`
  (`/Engine/EditorBlueprintResources/StandardMacros.IsValid` (`self.SaveGameInstance`)
    (:`Is Valid`
      _)
    (:`Is Not Valid`
      (bind _returnvalue (`GameplayStatics.CreateSaveGameObject` "/Game/Blueprints/Settings/DiceSaveGame.DiceSaveGame_C"))
      (set `self.SaveGameInstance` _returnvalue)))
  (bind _returnvalue_2 (`GameplayStatics.LoadGameFromSlot` "PlayedGamesInfo"))
  (bind _asdice_save_game (cast `/Game/Blueprints/Settings/DiceSaveGame` _returnvalue_2))
  (bind _output_get (set `self.SaveGameInstance` _asdice_save_game))
  (set `self.TotalGamesPlayed` (`/Game/Blueprints/Settings/DiceSaveGame.TotalGamesPlayed` _output_get))
  (set `self.ClassicGamesPlayed` (`/Game/Blueprints/Settings/DiceSaveGame.ClassicGamesPlayed` _output_get))
  (set `self.ModernGamesPlayedv2` (`/Game/Blueprints/Settings/DiceSaveGame.ModernGamesPlayedv2` _output_get))
  (set `self.ModernGamesPlayedv1` (`/Game/Blueprints/Settings/DiceSaveGame.ModernGamesPlayedv1` _output_get))
  (set `self.ClassicTutorialPlayed?` (`/Game/Blueprints/Settings/DiceSaveGame.ClassicTutorialPlayed?` _output_get))
  (set `self.ModernV1TutorialPlayed?` (`/Game/Blueprints/Settings/DiceSaveGame.ModernV1TutorialPlayed?` _output_get))
  (set `self.ModernV2TutorialPlayed?` (`/Game/Blueprints/Settings/DiceSaveGame.ModernV2TutorialPlayed?` _output_get)))

(event `ToText`
  (bind _output_get (set `self.Result` (`KismetStringLibrary.Concat_StrStr` (`self.Result`) (`KismetStringLibrary.Concat_StrStr` (`KismetStringLibrary.Conv_IntToString` (`self.Round`)) " | " (`KismetStringLibrary.Conv_IntToString` (`self.1`)) " " (`KismetStringLibrary.Conv_IntToString` (`self.2`)) " " (`KismetStringLibrary.Conv_IntToString` (`self.3`)) " " (`KismetStringLibrary.Conv_IntToString` (`self.4`)) " " (`KismetStringLibrary.Conv_IntToString` (`self.5`)) " " (`KismetStringLibrary.Conv_IntToString` (`self.6`)) " \n"))))
  (`VictoryBPFunctionLibrary.FileIO__SaveStringTextToFile` "C:\\Users\\Spidior\\Desktop" "Test.txt" _output_get true))