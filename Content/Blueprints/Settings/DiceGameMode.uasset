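; DiceGameMode is a game mode Blueprint that switches the on-screen UI between the Hero Presentation and Answer widgets.
; Each has its own show event, which creates the widget only if the cached reference is invalid, then reuses it.
; The event removes whatever CurrentUI holds from its parent, adds the requested widget to the viewport and records it as CurrentUI.
; BeginPlay, Tick and the construction script do nothing.
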(event `ShowHeroPresentation`
  (bind _currentui (`self.CurrentUI`))
  ;[1 1 1] Shows Hero Presentation UI
  (`/Engine/EditorBlueprintResources/StandardMacros.IsValid` (`self.HeroPresentationUI`)
    (:`Is Valid`
      _)
    (:`Is Not Valid`
      (bind _returnvalue (`|CreateWidget` "/Game/Blueprints/UI/HeroPresentation.HeroPresentation_C"))
      (bind _output_get (set `self.HeroPresentationUI` _returnvalue))))
  (`/Engine/EditorBlueprintResources/StandardMacros.IsValid` _currentui
    (:`Is Valid`
      (`Widget.RemoveFromParent` _currentui))
    (:`Is Not Valid`
      _))
  (`UserWidget.AddToViewport` _output_get 0)
  (set `self.CurrentUI` _output_get))

(event `ShowAnswerUI`
  (bind _currentui (`self.CurrentUI`))
  ;[1 1 1] Shows Answer UI
  (`/Engine/EditorBlueprintResources/StandardMacros.IsValid` (`self.AnswerUI`)
    (:`Is Valid`
      _)
    (:`Is Not Valid`
      (bind _returnvalue (`|CreateWidget` "/Game/Blueprints/UI/Answer.Answer_C"))
      (bind _output_get (set `self.AnswerUI` _returnvalue))))
  (`/Engine/EditorBlueprintResources/StandardMacros.IsValid` _currentui
    (:`Is Valid`
      (`Widget.RemoveFromParent` _currentui))
    (:`Is Not Valid`
      _))
  (`UserWidget.AddToViewport` _output_get 0)
  (set `self.CurrentUI` _output_get))

(fn `UserConstructionScript`)