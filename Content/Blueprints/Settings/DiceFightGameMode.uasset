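; DiceFightGameMode is the Dice Fight game mode, acting as a manager for full-screen UI widgets.
; Show events cover mode select, hero presentations, round countdown, loading, feedback, exit prompt and congratulations.
; Each event creates and caches its widget when invalid, then swaps it with CurrentUI in the viewport.
; The pause menu instead overlays the current screen, with separate show and hide events that toggle a Hidden flag.
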(event `ShowHeroPresentation`
  (bind _currentui (`self.CurrentUI`))
  ;[1 1 1] Shows Classic Hero Presentation UI
  (`/Engine/EditorBlueprintResources/StandardMacros.IsValid` null
    (:`Is Valid`
      _)
    (:`Is Not Valid`
      (bind _returnvalue (`|CreateWidget` "/Game/Blueprints/UI/ClassicHeroPresentation.ClassicHeroPresentation_C"))
      (bind _output_get (set `self.ClassicHeroPresentationUI` _returnvalue))))
  (`/Engine/EditorBlueprintResources/StandardMacros.IsValid` _currentui
    (:`Is Valid`
      (`Widget.RemoveFromParent` _currentui))
    (:`Is Not Valid`
      _))
  (`UserWidget.AddToViewport` _output_get 0)
  (set `self.CurrentUI` _output_get))

(event `ShowSelectModeUI`
  (bind _currentui (`self.CurrentUI`))
  ;[1 1 1] Shows Select Mode UI
  (`/Engine/EditorBlueprintResources/StandardMacros.IsValid` null
    (:`Is Valid`
      _)
    (:`Is Not Valid`
      (bind _returnvalue (`|CreateWidget` "/Game/Blueprints/UI/ModeSelect.ModeSelect_C"))
      (bind _output_get (set `self.ModeSelectUI` _returnvalue))))
  (`/Engine/EditorBlueprintResources/StandardMacros.IsValid` _currentui
    (:`Is Valid`
      (`Widget.RemoveFromParent` _currentui))
    (:`Is Not Valid`
      _))
  (`UserWidget.AddToViewport` _output_get 0)
  (set `self.CurrentUI` _output_get))

(event `ShowModernHeroPresentation`
  (bind _currentui (`self.CurrentUI`))
  ;[1 1 1] Showing Modern Hero Presentation UI
  (`/Engine/EditorBlueprintResources/StandardMacros.IsValid` (`self.ModernHeroPresentatioUI`)
    (:`Is Valid`
      _)
    (:`Is Not Valid`
      (bind _returnvalue (`|CreateWidget` "/Game/Blueprints/UI/ModeHeroPresentation.ModeHeroPresentation_C"))
      (bind _output_get (set `self.ModernHeroPresentatioUI` _returnvalue))))
  (`/Engine/EditorBlueprintResources/StandardMacros.IsValid` _currentui
    (:`Is Valid`
      (`Widget.RemoveFromParent` _currentui))
    (:`Is Not Valid`
      _))
  (`UserWidget.AddToViewport` _output_get 0)
  (set `self.CurrentUI` _output_get))

(event `ShowPauseMenuUI`
  ;[1 1 1] Showing Menu UI
  (`/Engine/EditorBlueprintResources/StandardMacros.IsValid` (`self.PauseMenuUI`)
    (:`Is Valid`
      _)
    (:`Is Not Valid`
      (bind _returnvalue (`|CreateWidget` "/Game/Blueprints/UI/PauseMenu.PauseMenu_C"))
      (bind _output_get (set `self.PauseMenuUI` _returnvalue))))
  (`UserWidget.AddToViewport` _output_get 0)
  (set `self.Hidden?` false))

(event `HidePauseMenuUI`
  (bind _pausemenuui (`self.PauseMenuUI`))
  ;[1 1 1] Hide Menu UI
  (`/Engine/EditorBlueprintResources/StandardMacros.IsValid` _pausemenuui
    (:`Is Valid`
      (if (`Widget.IsInViewport` _pausemenuui)
        (`Widget.RemoveFromParent` _pausemenuui)
        (set `self.Hidden?` true)))))

(event `ShowFeedbackUI`
  (bind _currentui (`self.CurrentUI`))
  ;[1 1 1] Show Feedback UI
  (`/Engine/EditorBlueprintResources/StandardMacros.IsValid` (`self.FeddbackUI`)
    (:`Is Valid`
      _)
    (:`Is Not Valid`
      (bind _returnvalue (`|CreateWidget` "/Game/Blueprints/UI/Feedback.Feedback_C"))
      (bind _output_get (set `self.FeddbackUI` _returnvalue))))
  (`/Engine/EditorBlueprintResources/StandardMacros.IsValid` _currentui
    (:`Is Valid`
      (`Widget.RemoveFromParent` _currentui))
    (:`Is Not Valid`
      _))
  (`UserWidget.AddToViewport` _output_get 0)
  (set `self.CurrentUI` _output_get))

(event `ShowRoundCountingdownUI`
  (bind _currentui (`self.CurrentUI`))
  ;[1 1 1] Showing Round Countindown UI
  (`/Engine/EditorBlueprintResources/StandardMacros.IsValid` (`self.RoundCountingdownUI`)
    (:`Is Valid`
      _)
    (:`Is Not Valid`
      (bind _returnvalue (`|CreateWidget` "/Game/Blueprints/UI/RoundCountdown.RoundCountdown_C"))
      (bind _output_get (set `self.RoundCountingdownUI` _returnvalue))))
  (`/Engine/EditorBlueprintResources/StandardMacros.IsValid` _currentui
    (:`Is Valid`
      (`Widget.RemoveFromParent` _currentui))
    (:`Is Not Valid`
      _))
  (`UserWidget.AddToViewport` _output_get 0)
  (set `self.CurrentUI` _output_get))

(event `ShowLoadingScreen`
  (bind _currentui (`self.CurrentUI`))
  ;[1 1 1] Showing Loading Screen UI
  (`/Engine/EditorBlueprintResources/StandardMacros.IsValid` (`self.LoadingScreenUI`)
    (:`Is Valid`
      _)
    (:`Is Not Valid`
      (bind _returnvalue (`|CreateWidget` "/Game/Blueprints/UI/LoadingScreen.LoadingScreen_C"))
      (bind _output_get (set `self.LoadingScreenUI` _returnvalue))))
  (`/Engine/EditorBlueprintResources/StandardMacros.IsValid` _currentui
    (:`Is Valid`
      (`Widget.RemoveFromParent` _currentui))
    (:`Is Not Valid`
      _))
  (`UserWidget.AddToViewport` _output_get 0)
  (set `self.CurrentUI` _output_get))

(event `ShowExitPrompt`
  (bind _currentui (`self.CurrentUI`))
  ;[1 1 1] Showing Exit Prompt
  (`/Engine/EditorBlueprintResources/StandardMacros.IsValid` (`self.ExitPromptUI`)
    (:`Is Valid`
      _)
    (:`Is Not Valid`
      (bind _returnvalue (`|CreateWidget` "/Game/Blueprints/UI/ExitPrompt.ExitPrompt_C"))
      (bind _output_get (set `self.ExitPromptUI` _returnvalue))))
  (`/Engine/EditorBlueprintResources/StandardMacros.IsValid` _currentui
    (:`Is Valid`
      (`Widget.RemoveFromParent` _currentui))
    (:`Is Not Valid`
      _))
  (`UserWidget.AddToViewport` _output_get 0)
  (set `self.CurrentUI` _output_get))

(event `ShowCongratulationUI`
  (bind _currentui (`self.CurrentUI`))
  ;[1 1 1] Showing Congratulation UI
  (`/Engine/EditorBlueprintResources/StandardMacros.IsValid` (`self.CongratulationUI`)
    (:`Is Valid`
      _)
    (:`Is Not Valid`
      (bind _returnvalue (`|CreateWidget` "/Game/Blueprints/UI/Congratulations.Congratulations_C"))
      (bind _output_get (set `self.CongratulationUI` _returnvalue))))
  (`/Engine/EditorBlueprintResources/StandardMacros.IsValid` _currentui
    (:`Is Valid`
      (`Widget.RemoveFromParent` _currentui))
    (:`Is Not Valid`
      _))
  (`UserWidget.AddToViewport` _output_get 0)
  (set `self.CurrentUI` _output_get))

(fn `UserConstructionScript`)